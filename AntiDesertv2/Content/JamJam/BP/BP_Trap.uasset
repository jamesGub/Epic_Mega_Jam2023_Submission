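; BP_Trap is a trap actor that deals continuous damage to pawns inside its box collider.
; Box overlap events add entering pawns to a DamagingActors array, remove leaving actors, and set a TrapUp flag through DoOnce nodes.
; Tick applies DamageFactor scaled by delta time to each tracked actor and prints a debug string.
; ActivateTrap toggles the collider between query-only and no collision.
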(event OnComponentBeginOverlap(Box)
  (params (OverlappedComponent :type Primitive%20Component%20Object%20Reference) (OtherActor :type Actor%20Object%20Reference) (OtherComp :type Primitive%20Component%20Object%20Reference) (OtherBodyIndex :type Integer) (bFromSweep :type Boolean) (SweepResult :type Hit%20Result%20Structure%20%28by%20ref%29))
  ;[0.4052 0.01531 0 0.483] Damage
  (Utilities|Casting|CastToPawn OtherActor)
  (Utilities|Array|Add (Variables|Default|GetDamagingActors) OtherActor)
  (Utilities|FlowControl|DoOnce false
    (:Completed
      (Variables|Default|SetTrapUp true))))

(event OnComponentEndOverlap(Box)
  (params (OverlappedComponent :type Primitive%20Component%20Object%20Reference) (OtherActor :type Actor%20Object%20Reference) (OtherComp :type Primitive%20Component%20Object%20Reference) (OtherBodyIndex :type Integer))
  ;[0.4052 0.01531 0 0.483] Damage
  (Utilities|Array|RemoveItem (Variables|Default|GetDamagingActors) OtherActor)
  (Utilities|DoOnce true
    (:Completed
      (Variables|Default|SetTrapUp true))))

(event Custom|ActivateTrap
  (params (activate :type Boolean))
  (bind _boxcollider (Variables|Default|GetBoxCollider))
  (if activate
    (Collision|SetCollisionEnabled _boxcollider "QueryOnly")
    (else
      (Collision|SetCollisionEnabled _boxcollider "NoCollision"))))

(event Custom|InflictDamage
  (params (deltaTime :type Float%20%28double-precision%29))
  ;[0.4052 0.01531 0 0.483] Damage
  (for _array_element (Variables|Default|GetDamagingActors)
    (Game|Damage|ApplyDamage _array_element (* (Variables|Default|GetDamageFactor) deltaTime) 0 0 "/Script/Engine.DamageType")
    (Development|PrintString "Hitting")))

(event EventBeginPlay)

(event Collision|EventActorBeginOverlap
  (params (OtherActor :type Actor%20Object%20Reference)))

(event EventTick
  (params (DeltaSeconds :type Float%20%28single-precision%29))
  (CallFunction|InflictDamage DeltaSeconds))

(fn ConstructionScript)