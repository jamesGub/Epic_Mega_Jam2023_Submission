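; Weather actor that shifts the level between a dark and a light atmosphere, alternating on a short timed sequence from BeginPlay.
; Each change stores targets and enables Tick, which interpolates at constant speed and disables itself once exposure nears its target.
; SetAtmosphere applies the values to Sky Atmosphere Rayleigh scattering, post-process exposure compensation and a dynamic volumetric cloud material's density.
; Darken and Lighten events apply either preset instantly.
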(event Custom|Darken
  (CallFunction|SetAtmosphere "(R=0.044515,G=0.106837,B=0.260417,A=1.000000)" -1.0 0.05))

(event Custom|Lighten
  (CallFunction|SetAtmosphere "(R=0.310602,G=0.450450,B=0.921875,A=1.000000)" 0.5 0.3))

(event Custom|SetAtmosphereTargetParam
  (params (Target%20Cloud%20Density_0 :type Float%20%28single-precision%29) (Target%20Exposure%20Compensation_0 :type Float%20%28single-precision%29) (Target%20Rayleigh%20Scattering_0 :type Linear%20Color%20Structure))
  (Variables|AtmosphereValues|SetTarget%20Cloud%20Density_0 Target%20Cloud%20Density_0)
  (Variables|AtmosphereValues|SetTarget%20Exposure%20Compensation_0 Target%20Exposure%20Compensation_0)
  (Variables|AtmosphereValues|SetTarget%20Rayleigh%20Scattering_0 Target%20Rayleigh%20Scattering_0)
  (Actor|Tick|SetActorTickEnabled true))

(event EventBeginPlay
  (Utilities|FlowControl|Delay 5.0)
  (CallFunction|SetAtmosphereTargetParam 0.05 -1.0 "(R=0.043137,G=0.105882,B=0.258824,A=1.000000)")
  (Utilities|FlowControl|Delay 5.0)
  (CallFunction|SetAtmosphereTargetParam 0.3 0.5 "(R=0.309804,G=0.450980,B=0.921569,A=1.000000)")
  (Utilities|FlowControl|Delay 5.0)
  (CallFunction|SetAtmosphereTargetParam 0.05 -1.0 "(R=0.043137,G=0.105882,B=0.258824,A=1.000000)")
  (Utilities|FlowControl|Delay 5.0)
  (CallFunction|SetAtmosphereTargetParam 0.3 0.5 "(R=0.309804,G=0.450980,B=0.921569,A=1.000000)")
  (Utilities|FlowControl|Delay 5.0)
  (CallFunction|SetAtmosphereTargetParam 0.05 -1.0 "(R=0.043137,G=0.105882,B=0.258824,A=1.000000)")
  (Utilities|FlowControl|Delay 5.0)
  (CallFunction|SetAtmosphereTargetParam 0.3 0.5 "(R=0.309804,G=0.450980,B=0.921569,A=1.000000)")
  (Utilities|FlowControl|Delay 5.0)
  (CallFunction|SetAtmosphereTargetParam 0.05 -1.0 "(R=0.043137,G=0.105882,B=0.258824,A=1.000000)")
  (Utilities|FlowControl|Delay 5.0)
  (CallFunction|SetAtmosphereTargetParam 0.3 0.5 "(R=0.309804,G=0.450980,B=0.921569,A=1.000000)"))

(event Collision|EventActorBeginOverlap
  (params (OtherActor :type Actor%20Object%20Reference)))

(event EventTick
  (params (DeltaSeconds :type Float%20%28single-precision%29))
  (bind _returnvalue (Math|Float|MakeLiteralFloat 1.0))
  (bind _exposure_compensation (Variables|AtmosphereValues|GetExposure%20Compensation))
  (bind _target_exposure_compensation_0 (Variables|AtmosphereValues|GetTarget%20Exposure%20Compensation_0))
  (CallFunction|SetAtmosphere (CallFunction|ColorInterptoConstant (Variables|AtmosphereValues|GetRayleigh%20Scattering) (Variables|AtmosphereValues|GetTarget%20Rayleigh%20Scattering_0) _returnvalue) (Math|Interpolation|FInterptoConstant _exposure_compensation _target_exposure_compensation_0 DeltaSeconds _returnvalue) (Math|Interpolation|FInterptoConstant (Variables|AtmosphereValues|GetCloud%20Density) (Variables|AtmosphereValues|GetTarget%20Cloud%20Density_0) DeltaSeconds _returnvalue))
  (Actor|Tick|SetActorTickEnabled (not (Math|Float|NearlyEqual(Float) _exposure_compensation _target_exposure_compensation_0 0.05))))

(fn ConstructionScript)

(fn SetAtmosphere
  (params (RayleighScattering%20 :type Linear%20Color%20Structure) (Exposure%20Compensation :type Float%20%28single-precision%29) (CloudDensity :type Float%20%28single-precision%29))
  (Variables|AtmosphereValues|SetCloud%20Density CloudDensity)
  (Variables|AtmosphereValues|SetExposure%20Compensation Exposure%20Compensation)
  (Variables|AtmosphereValues|SetRayleigh%20Scattering RayleighScattering%20)
  (Class|SkyAtmosphereComponent|SetRayleighScattering (Variables|/Script/Engine.SkyAtmosphere|GetSkyAtmosphereComponent (Variables|Default|GetSkyAtmosphere)) RayleighScattering%20)
  (Utilities|Struct|SetmembersinPostProcessSettings (Variables|/Script/Engine.PostProcessVolume|GetSettings (Variables|Default|GetPostProcessVolume)) Exposure%20Compensation)
  (Variables|Default|GetCloudMat
    (:then
      _)
    (:else
      (bind _returnvalue (Rendering|Material|CreateDynamicMaterialInstance "/Engine/EngineSky/VolumetricClouds/m_SimpleVolumetricCloud_Inst.m_SimpleVolumetricCloud_Inst" "m_SimpleVolumetricCloud_Inst" "None" :!class /Script/Engine.KismetMaterialLibrary))
      (bind _output_get (Variables|Default|SetCloudMat _returnvalue))))
  (Rendering|Material|SetMaterial (Variables|/Script/Engine.VolumetricCloud|GetVolumetricCloudComponent (Variables|Default|GetVolumetricClouds)) _output_get)
  (Rendering|Material|SetScalarParameterValue _output_get "DensityOffset" CloudDensity :!class /Script/Engine.MaterialInstanceDynamic))

(fn ColorInterptoConstant
  (params (InColor :type Linear%20Color%20Structure) (InColor2 :type Linear%20Color%20Structure) (InputPin :type Float%20%28double-precision%29))
  (bind (_r _g _b _a) (Math|Color|BreakColor InColor))
  (bind _returnvalue (Utilities|Time|GetWorldDeltaSeconds))
  (bind (_r_2 _g_2 _b_2 _a_2) (Math|Color|BreakColor InColor2))
  (return (Utilities|Struct|MakeLinearColor (Math|Interpolation|FInterptoConstant _r _r_2 _returnvalue InputPin) (Math|Interpolation|FInterptoConstant _g _g_2 _returnvalue InputPin) (Math|Interpolation|FInterptoConstant _b _b_2 _returnvalue InputPin) (Math|Interpolation|FInterptoConstant _a _a_2 _returnvalue InputPin))))