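; Resizable electric trap actor that deals damage over time to pawns standing inside its box collider.
; The construction script scales the cube, collider and Niagara-style beam effect parameters from Size relative to RefSize.
; Overlap events track pawns in a list, and Tick applies damage scaled by delta time to each.
; ActivateTrap toggles collider collision and zeroes or restores the effect's spawn count.
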(event OnComponentBeginOverlap(BoxCollider)
  (params (OverlappedComponent :type Primitive%20Component%20Object%20Reference) (OtherActor :type Actor%20Object%20Reference) (OtherComp :type Primitive%20Component%20Object%20Reference) (OtherBodyIndex :type Integer) (bFromSweep :type Boolean) (SweepResult :type Hit%20Result%20Structure%20%28by%20ref%29))
  ;[0.4052 0.01531 0 0.483] Damage
  (Utilities|Casting|CastToPawn OtherActor)
  (Utilities|Array|Add (Variables|Default|GetDamagingActors) OtherActor))

(event OnComponentEndOverlap(BoxCollider)
  (params (OverlappedComponent :type Primitive%20Component%20Object%20Reference) (OtherActor :type Actor%20Object%20Reference) (OtherComp :type Primitive%20Component%20Object%20Reference) (OtherBodyIndex :type Integer))
  ;[0.4052 0.01531 0 0.483] Damage
  (Utilities|Array|RemoveItem (Variables|Default|GetDamagingActors) OtherActor))

(event Custom|ActivateTrap
  (params (activate :type Boolean))
  (bind _boxcollider (Variables|Default|GetBoxCollider))
  (if activate
    (Collision|SetCollisionEnabled _boxcollider "QueryOnly")
    (CallFunction|ResetSpawnCount)
    (else
      (Collision|SetCollisionEnabled _boxcollider "NoCollision")
      (Class|NiagaraComponent|SetVariableInt (Variables|Default|GetElectricBlock) "MaxSpawnCount"))))

(event Custom|InflictDamage
  (params (deltaTime :type Float%20%28double-precision%29))
  ;[0.4052 0.01531 0 0.483] Damage
  (for _array_element (Variables|Default|GetDamagingActors)
    (Game|Damage|ApplyDamage _array_element (* (Variables|Default|GetDamageFactor) deltaTime) 0 0)
    (Development|PrintString "Hitting")))

(event Custom|ResetSpawnCount
  (Class|NiagaraComponent|SetVariableInt (Variables|Default|GetElectricBlock) "MaxSpawnCount" (Math|Float|Truncate (* (Class|KismetMathLibrary|GetMin2D (/ (Variables|Default|GetSize) (Variables|Default|GetRefSize))) 5e+01))))

(event EventBeginPlay)

(event Collision|EventActorBeginOverlap
  (params (OtherActor :type Actor%20Object%20Reference)))

(event EventTick
  (params (DeltaSeconds :type Float%20%28single-precision%29))
  (CallFunction|InflictDamage DeltaSeconds))

(fn ConstructionScript
  (bind _cube (Variables|Default|GetCube))
  (bind _boxcollider (Variables|Default|GetBoxCollider))
  (bind _size (Variables|Default|GetSize))
  (bind _size_2 (Variables|Default|GetSize))
  (bind _returnvalue (Transformation|GetRelativeTransform _boxcollider))
  (bind _returnvalue_2 (Transformation|GetRelativeTransform _cube))
  (bind _returnvalue_3 (* _size "(X=-1.000000,Y=-1.000000)"))
  (LocalVariables|SetScaleFactor (/ (Variables|Default|GetSize) (Variables|Default|GetRefSize)))
  (Transformation|SetRelativeScale3D _cube (Math|Vector|MakeVector (* (.x (.scale _returnvalue_2)) (.x (LocalVariables|GetScaleFactor))) (* (.y (.scale _returnvalue_2)) (.y (LocalVariables|GetScaleFactor))) (.z (.scale _returnvalue_2))))
  (Niagara|SetNiagaraVariable(Vector3) (Variables|Default|GetElectricBlock) "MinEnd" (Math|Vector|MakeVector (.x _returnvalue_3) (.y _returnvalue_3) 0.0))
  (Niagara|SetNiagaraVariable(Vector3) (Variables|Default|GetElectricBlock) "MaxEnd" (Math|Vector|MakeVector (.x _size_2) (.y _size_2) 0.0))
  (Niagara|SetNiagaraVariable(Float) (Variables|Default|GetElectricBlock) "MaxBeamTangent" (* (Class|KismetMathLibrary|GetMin2D (LocalVariables|GetScaleFactor)) 0.2))
  (Class|NiagaraComponent|SetVariableInt (Variables|Default|GetElectricBlock) "MaxSpawnCount" (Math|Float|Truncate (* (Class|KismetMathLibrary|GetMin2D (LocalVariables|GetScaleFactor)) 5e+01)))
  (Transformation|SetRelativeScale3D _boxcollider (Math|Vector|MakeVector (* (.x (.scale _returnvalue)) (.x (LocalVariables|GetScaleFactor))) (* (.y (.scale _returnvalue)) (.y (LocalVariables|GetScaleFactor))) (.z (.scale _returnvalue)))))