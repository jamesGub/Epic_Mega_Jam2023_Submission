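; Laser trap actor that fires a beam along its forward vector and damages pawns caught in it over time.
; Each tick the beam grows at a set velocity up to a max distance, clipped by a visibility line trace that drives the beam end and impact effect.
; A capsule collider is resized to the beam, tracking overlapping pawns for frame-scaled damage.
; The construction script applies color and previews full length.
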(event OnComponentBeginOverlap(Collider)
  (params (OverlappedComponent :type Primitive%20Component%20Object%20Reference) (OtherActor :type Actor%20Object%20Reference) (OtherComp :type Primitive%20Component%20Object%20Reference) (OtherBodyIndex :type Integer) (bFromSweep :type Boolean) (SweepResult :type Hit%20Result%20Structure%20%28by%20ref%29))
  ;[0.4052 0.01531 0 0.483] Damage
  (Utilities|Casting|CastToPawn OtherActor)
  (Utilities|Array|Add (Variables|Default|GetDamagingActors) OtherActor))

(event OnComponentEndOverlap(Collider)
  (params (OverlappedComponent :type Primitive%20Component%20Object%20Reference) (OtherActor :type Actor%20Object%20Reference) (OtherComp :type Primitive%20Component%20Object%20Reference) (OtherBodyIndex :type Integer))
  ;[0.4052 0.01531 0 0.483] Damage
  (Utilities|Array|RemoveItem (Variables|Default|GetDamagingActors) OtherActor))

(event Custom|InflictDamage
  (params (deltaTime :type Float%20%28double-precision%29))
  ;[0.4052 0.01531 0 0.483] Damage
  (for _array_element (Variables|Default|GetDamagingActors)
    (Game|Damage|ApplyDamage _array_element (* (Variables|Default|GetDamageFactor) deltaTime) 0 0)))

(event EventBeginPlay)

(event Collision|EventActorBeginOverlap
  (params (OtherActor :type Actor%20Object%20Reference)))

(event EventTick
  (params (DeltaSeconds :type Float%20%28single-precision%29))
  (bind _returnvalue (Transformation|GetActorLocation))
  (bind _maxdistance (Variables|Default|GetMaxDistance))
  (CallFunction|InflictDamage DeltaSeconds)
  (Variables|Default|SetCurrentDistance (Math|Float|SelectFloat _maxdistance (+ (* DeltaSeconds (Variables|Default|GetLaserVelocity)) (Variables|Default|GetCurrentDistance)) (> (+ (* DeltaSeconds (Variables|Default|GetLaserVelocity)) (Variables|Default|GetCurrentDistance)) _maxdistance)))
  (bind _outhit (Collision|LineTraceByChannel _returnvalue (+ _returnvalue (* (Transformation|GetActorForwardVector) (Variables|Default|GetCurrentDistance))) "TraceTypeQuery1" false 0 "None"))
  (if (.bblockinghit _outhit)
    (Variables|Default|SetCurrentDistance (.distance _outhit)))
  (Effects|Components|ParticleSystem|SetVectorParameter (Variables|Default|GetLaser) "LaserEnd" (Math|Vector|SelectVector (.location _outhit) (+ _returnvalue (* (Transformation|GetActorForwardVector) (Variables|Default|GetCurrentDistance))) (.bblockinghit _outhit)))
  (Rendering|SetVisibility (Variables|Default|GetLaserImpact) (.bblockinghit _outhit) false)
  (Transformation|SetWorldLocation (Variables|Default|GetLaserImpact) (Math|Vector|SelectVector (.location _outhit) (+ _returnvalue (* (Transformation|GetActorForwardVector) (Variables|Default|GetCurrentDistance))) (.bblockinghit _outhit)) false false)
  (Components|Capsule|SetCapsuleHalfHeight (Variables|Default|GetCollider) (/ (Variables|Default|GetCurrentDistance) 2.0) true)
  (Transformation|SetWorldLocation (Variables|Default|GetCollider) (+ (Transformation|GetActorLocation) (* (Transformation|GetActorForwardVector) (/ (Variables|Default|GetCurrentDistance) 2.0))) false false))

(fn ConstructionScript
  (Niagara|SetNiagaraVariable(LinearColor) (Variables|Default|GetLaserImpact) "Color" (Variables|Default|GetColor))
  (Effects|Components|ParticleSystem|SetVectorParameter (Variables|Default|GetLaser) "LaserEnd" (+ (Transformation|GetActorLocation) (* (Transformation|GetActorForwardVector) (Variables|Default|GetMaxDistance)))))