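; CollectablePotion is a collectable pickup that restores health to the player.
; It overrides the inherited Collect event, running the parent logic before casting player 0's character to BP_ThirdPersonCharacter and calling Cure with HealthAmount.
; The healing always targets that first player character, and the Blueprint adds no overlap, tick or construction logic of its own.
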(event EventBeginPlay
  (|CallParentFunction) ; 此节点被禁用，将不会被调用。\n从引脚连出引线来编译功能。
)

(event Collision|EventActorBeginOverlap
  (params (OtherActor :type Actor%20Object%20Reference))
  (|CallParentFunction OtherActor) ; 此节点被禁用，将不会被调用。\n从引脚连出引线来编译功能。
)

(event EventTick
  (params (DeltaSeconds :type Float%20%28single-precision%29))
  (|CallParentFunction DeltaSeconds) ; 此节点被禁用，将不会被调用。\n从引脚连出引线来编译功能。
)

(event EventCollect
  (|CallParentFunction)
  (bind _asbp_third_person_character (Utilities|Casting|CastToBP_ThirdPersonCharacter (Game|GetPlayerCharacter 0)))
  (Default|Cure _asbp_third_person_character (Variables|Default|GetHealthAmount)))

(fn ConstructionScript
  (|CallParentFunction))