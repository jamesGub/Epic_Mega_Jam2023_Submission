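; BP_SandPile2 is a sand pile actor that briefly shows a sand display UI when another actor overlaps it.
; The overlap event adds a widget to the viewport, waits two seconds, removes all widgets, then recreates and re-adds WB_HUD before calling the parent overlap handler.
; The overlapping actor is not filtered, so any overlap triggers the sequence and rebuilds the HUD.
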(event EventBeginPlay
  (|CallParentFunction) ; This node is disabled and will not be called.\nDrag off pins to build functionality.
)

(event Collision|EventActorBeginOverlap
  (params (OtherActor :type Actor%20Object%20Reference))
  ;[0.5588 1 0.237] Sand display UI
  (bind _returnvalue (UserInterface|CreateWidget (Variables|Default|GetClass)))
  (UserInterface|Viewport|AddtoViewport _returnvalue 0)
  (Utilities|FlowControl|Delay 2.0)
  (Viewport|RemoveAllWidgets)
  (bind _returnvalue_2 (UserInterface|CreateWidget "/Game/UI/Menus/HUD/WB_HUD.WB_HUD_C"))
  (UserInterface|Viewport|AddtoViewport _returnvalue_2 0)
  (|CallParentFunction OtherActor))

(event EventTick
  (params (DeltaSeconds :type Float%20%28single-precision%29))
  (|CallParentFunction DeltaSeconds) ; This node is disabled and will not be called.\nDrag off pins to build functionality.
)

(fn ConstructionScript
  (|CallParentFunction))