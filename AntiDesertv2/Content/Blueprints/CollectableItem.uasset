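; Collectable item actor with a sphere trigger that can be switched on or off for interaction and a Collect event that destroys it.
; Sphere overlaps drive EnableCollection, and leaving removes the UI prompt built from "Collect" and the lowercased item name.
; Entering is unfinished: it stops after a player pawn cast flagged for a post-merge fix, leaving the prompt display disconnected.
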(event OnComponentBeginOverlap(SphereCollider)
  (params (OverlappedComponent :type Primitive%20Component%20Object%20Reference) (OtherActor :type Actor%20Object%20Reference) (OtherComp :type Primitive%20Component%20Object%20Reference) (OtherBodyIndex :type Integer) (bFromSweep :type Boolean) (SweepResult :type Hit%20Result%20Structure%20%28by%20ref%29))
  (CallFunction|EnableCollection true))

(event OnComponentEndOverlap(SphereCollider)
  (params (OverlappedComponent :type Primitive%20Component%20Object%20Reference) (OtherActor :type Actor%20Object%20Reference) (OtherComp :type Primitive%20Component%20Object%20Reference) (OtherBodyIndex :type Integer))
  (CallFunction|EnableCollection false))

(event Custom|EnableCollection
  (params (Enable :type Boolean))
  (if Enable
    ;[1 1 1] Needs to be fixed after mertge
    (Utilities|Casting|CastTo (Game|Player|GetPlayerPawn 0))
    (else
      (CallFunction|ShowCollectionInstruction false))))

(event Custom|EnableInteraction
  (params (enable :type Boolean))
  (bind _spherecollider (Variables|Default|GetSphereCollider))
  (if enable
    (Collision|SetCollisionEnabled _spherecollider "QueryOnly")
    (else
      (Collision|SetCollisionEnabled _spherecollider "NoCollision"))))

(event Custom|ShowCollectionInstruction
  (params (show :type Boolean))
  ;[0.2344 0.2344 0.2344] Show instruction to collect item in the UI
  (if show
    (bind _returnvalue (UserInterface|CreateWidget 0))
    (Variables|Default|SetInstructionText _returnvalue (Utilities|String|Append (Utilities|String|MakeLiteralString "Collect ") (Utilities|String|ToLower (Variables|Default|GetItemName))))
    (UserInterface|Viewport|AddtoViewport _returnvalue 0)
    (elif (Utilities|IsValid _returnvalue)
      (Widget|RemovefromParent _returnvalue))))

(event Custom|Collect
  (Actor|DestroyActor))

(fn ConstructionScript)