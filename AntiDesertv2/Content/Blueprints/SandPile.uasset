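; Sand pile actor that hides a collectable, spawned at BeginPlay with interaction disabled, until blown away.
; Overlap with a BlowingCollider drives sand particles horizontally away from it and plays a timeline that scales the pile.
; Ending the overlap stops the particles and pauses the timeline, so blowing resumes from the same point.
; Once scale drops to BlowEndRatio or below, the collectable becomes interactable.
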(event OnComponentEndOverlap(SphereCollider)
  (params (OverlappedComponent :type Primitive%20Component%20Object%20Reference) (OtherActor :type Actor%20Object%20Reference) (OtherComp :type Primitive%20Component%20Object%20Reference) (OtherBodyIndex :type Integer))
  (if (Class|GameplayStatics|ObjectIsA OtherActor "/Game/Blueprints/BlowingCollider.BlowingCollider_C")
    (CallFunction|StopBlow)))

(event OnComponentBeginOverlap(SphereCollider)
  (params (OverlappedComponent :type Primitive%20Component%20Object%20Reference) (OtherActor :type Actor%20Object%20Reference) (OtherComp :type Primitive%20Component%20Object%20Reference) (OtherBodyIndex :type Integer) (bFromSweep :type Boolean) (SweepResult :type Hit%20Result%20Structure%20%28by%20ref%29))
  (if (Class|GameplayStatics|ObjectIsA OtherActor "/Game/Blueprints/BlowingCollider.BlowingCollider_C")
    (CallFunction|Blow (Math|Vector|Normalize (Math|Vector|ProjectVectorontoPlane (- (Transformation|GetActorLocation) (Transformation|GetActorLocation OtherActor)) "0.000000,0.000000,1.000000")))))

(event Custom|Blow
  (params (blowDirection :type Vector :default "0.000000,0.000000,0.000000"))
  (bind _blownsandeffect (Variables|Default|GetBlownSandEffect))
  ;[1 1 1] Be blown behaviour
  (Niagara|SetNiagaraVariable(Float) _blownsandeffect "spawnRate" 2e+03)
  (Niagara|SetNiagaraVariable(Vector3) _blownsandeffect "BlowDirection" blowDirection)
  (Niagara|SetNiagaraVariable(Float) _blownsandeffect "bigSpawnRate" 1e+02)
  (Components|Timeline|SetPlayRate (Variables|Default|GetBlow%20Timeline) 0.2)
  (bind _scale (Timeline|Blow%20Timeline Play)
    (:Update
      (Transformation|SetRelativeScale3D (Variables|Default|GetDefaultSceneRoot) (Math|Conversions|ToVector(Float) _scale))
      (if (<= _scale (Variables|Default|GetBlowEndRatio))
        (CallFunction|BlowEnd)))))

(event Custom|StopBlow
  (bind _blownsandeffect (Variables|Default|GetBlownSandEffect))
  ;[1 1 1] Be blown behaviour
  (Niagara|SetNiagaraVariable(Float) _blownsandeffect "spawnRate" 0.0)
  (Niagara|SetNiagaraVariable(Float) _blownsandeffect "bigSpawnRate" 0.0)
  (bind _scale (Timeline|Blow%20Timeline Stop)
    (:Update
      (Transformation|SetRelativeScale3D (Variables|Default|GetDefaultSceneRoot) (Math|Conversions|ToVector(Float) _scale))
      (if (<= _scale (Variables|Default|GetBlowEndRatio))
        (CallFunction|BlowEnd)))))

(event Custom|BlowEnd
  (bind _collectableinstance (Variables|Default|GetCollectableInstance))
  (if (Utilities|IsValid _collectableinstance)
    (Default|EnableInteraction _collectableinstance true)))

(event EventBeginPlay
  (CallFunction|StopBlow)
  (bind _returnvalue (Game|SpawnActorfromClass (Variables|Default|GetCollectableItem) (Transformation|GetWorldTransform (Variables|Default|GetDefaultSceneRoot)) "Undefined" "MultiplyWithRoot" 0 0))
  (bind _output_get (Variables|Default|SetCollectableInstance _returnvalue))
  (Default|EnableInteraction _output_get false))

(event Collision|EventActorBeginOverlap
  (params (OtherActor :type Actor%20Object%20Reference)))

(event EventTick
  (params (DeltaSeconds :type Float%20%28single-precision%29)))

(fn ConstructionScript)