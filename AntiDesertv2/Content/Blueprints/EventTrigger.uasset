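; EventTrigger is a trigger volume actor that starts dialogue and an optional cinematic when the player enters it.
; Its Box overlap checks for player pawn 0, calls TriggerEvent, then destroys the actor if OnlyOneUse is set.
; TriggerEvent sends DialogueText to the GameManager's DialogueManager child actor as beeping, player-blocking talk.
; It also plays CinematicSequence, if valid, through a newly created level sequence player, without waiting for the dialogue to finish.
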(event OnComponentBeginOverlap(Box)
  (params (OverlappedComponent :type Primitive%20Component%20Object%20Reference) (OtherActor :type Actor%20Object%20Reference) (OtherComp :type Primitive%20Component%20Object%20Reference) (OtherBodyIndex :type Integer) (bFromSweep :type Boolean) (SweepResult :type Hit%20Result%20Structure%20%28by%20ref%29))
  (if (== (Game|Player|GetPlayerPawn 0) OtherActor)
    (CallFunction|TriggerEvent)
    (if (Variables|Default|GetonlyOneUse)
      (Actor|DestroyActor))))

(event Custom|TriggerEvent
  (bind _cinematicsequence (Variables|Default|GetcinematicSequence))
  (Utilities|FlowControl|Sequence
    (:then_0
      ;[1 1 1] Dialog
      (bind _asdialogue_manager (Utilities|Casting|CastToDialogueManager (Variables|/Script/Engine.ChildActorComponent|GetChildActor (Variables|/Game/Blueprints/GameManager.GameManager_C|GetDialogueManager (Variables|Default|GetGameManager)))))
      (Default|Talk _asdialogue_manager (Variables|Default|GetdialogueText) true true))
    (:then_1
      ;[1 1 1] Cinematic sequence
      (if (Utilities|IsValid _cinematicsequence)
        (bind _outactor (Sequencer|Player|CreateLevelSequencePlayer _cinematicsequence))
        (Sequencer|Player|Play (Variables|/Script/LevelSequence.LevelSequenceActor|GetSequencePlayer _outactor) :!class /Script/MovieScene.MovieSceneSequencePlayer)))))

(event EventBeginPlay)

(event Collision|EventActorBeginOverlap
  (params (OtherActor :type Actor%20Object%20Reference)))

(event EventTick
  (params (DeltaSeconds :type Float%20%28single-precision%29)))

(fn ConstructionScript)